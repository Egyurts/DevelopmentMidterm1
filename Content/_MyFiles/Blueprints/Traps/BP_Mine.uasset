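; BP_Mine is a trap actor that damages the player and explodes on contact.
; When ExplosionCollisionArea begins an overlap, it checks that the other actor is the player 0 character, cast to BP_ThirdPersonCharacter, so other actors are ignored.
; It then passes Damage to that character's DamageFunction, spawns the SimpleExplosion effect at MineBody's location and destroys itself.
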(event `self.Explosion Collision Area.OnComponentBeginOverlap`
  (params (OverlappedComponent :type "PrimitiveComponent Object Reference") (OtherActor :type "Actor Object Reference") (OtherComp :type "PrimitiveComponent Object Reference") (OtherBodyIndex :type Integer) (bFromSweep :type Boolean) (SweepResult :type "HitResult Structure (by ref)"))
  (bind _asbp_third_person_character (cast `/Game/ThirdPerson/Blueprints/BP_ThirdPersonCharacter` (`GameplayStatics.GetPlayerCharacter` 0)))
  (if (== _asbp_third_person_character OtherActor)
    (`/Game/ThirdPerson/Blueprints/BP_ThirdPersonCharacter.Damage Function` _asbp_third_person_character (`KismetMathLibrary.Conv_IntToDouble` (`self.Damage`)))
    (`NiagaraFunctionLibrary.SpawnSystemAtLocation` "/Niagara/DefaultAssets/Templates/Systems/SimpleExplosion.SimpleExplosion" (`SceneComponent.K2_GetComponentLocation` (`self.MineBody`)))
    (`self.K2_DestroyActor`)))

(fn `UserConstructionScript`)