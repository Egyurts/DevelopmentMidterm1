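; BP_CogPuzzle is a rotating dial puzzle that opens a linked door when the Dugme component reaches a target yaw.
; Each InteractwithPuzzle call steps the passed component five degrees left or right, based on Dugme's current rotation.
; A tolerance check against RotationForActivatingDoor turns the Gosterge indicator green, plays a sound and calls OpenDoor on BPDoor; otherwise the indicator turns red.
; GetInteractState always returns false.
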(event `self.ReceiveBeginPlay`
  (`SceneComponent.K2_SetRelativeRotation` (`self.Dugme`) (`KismetMathLibrary.MakeRotator` 0.0) false false))

(event `/Game/_MyFiles/Blueprints/Interfaces/BPI_Interact.InteractWithPuzzle`
  (params (Component :type "PrimitiveComponent Object Reference") (RotateLeft :type Boolean))
  (bind (_relativerotation_roll _relativerotation_pitch _relativerotation_yaw) (`KismetMathLibrary.BreakRotator` (`SceneComponent.RelativeRotation` (`self.Dugme`))))
  (`SceneComponent.K2_SetRelativeRotation` Component (`KismetMathLibrary.MakeRotator` _relativerotation_roll _relativerotation_pitch (+ _relativerotation_yaw (select `bool` RotateLeft :`false` 5.0 :`true` -5.0))) false false)
  (if (== (`SceneComponent.RelativeRotation` (`self.Dugme`)) (`KismetMathLibrary.MakeRotator` 0.0 0.0 (`self.RotationForActivatingDoor`)) :`ErrorTolerance` 4.0)
    (`GameplayStatics.PlaySound2D` null 0.2 1.0 0.0 null null)
    (`PrimitiveComponent.SetMaterial` (`self.Gosterge`) 0 "/Game/_MyFiles/Materials/M_CogGreen.M_CogGreen")
    (`/Game/_MyFiles/Blueprints/BP_CogDoor.Open Door` (`self.BP_Door`))
    (else
      (`PrimitiveComponent.SetMaterial` (`self.Gosterge`) 0 "/Game/_MyFiles/Materials/M_CogRed.M_CogRed"))))

(fn `GetInteractState`
  (returns (DidInteract :type Boolean))
  (return false))

(fn `UserConstructionScript`)