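; Modular maze cell actor that builds one grid tile of a labyrinth in its Construction Script.
; It scales the floor from GridSize, then uses macros to add flagged walls, corner pillars and an optional ceiling with configurable spotlight.
; MazeTypeEnum selects a child pickup or hazard, with a random chance for med kits and random placement for mines.
; Two events switch the spotlight red or green at runtime.
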(event `Change Light Color(Red)`
  (bind _spotlight (`self.Spotlight`)
    (:`then`
      (`LightComponent.SetLightColor` _spotlight (struct :`R` 1.0 :`A` 1.0) true))
    (:`else`)))

(event `Change Light Color(Green)`
  (bind _spotlight (`self.Spotlight`)
    (:`then`
      (`LightComponent.SetLightColor` _spotlight (struct :`R` 0.07461 :`G` 1.0 :`A` 1.0) true))
    (:`else`)))

(fn `UserConstructionScript`
  (locals (WallLength :type "Float (double-precision)") (WallThickness :type "Float (double-precision)"))
  (bind _floor (`self.Floor`))
  (bind _gridsize (`self.GridSize`))
  (bind _walllength (`local.WallLength`))
  (bind _floor_2 (`self.Floor`))
  (bind _floor_3 (`self.Floor`))
  (bind _returnvalue_location (`KismetMathLibrary.BreakTransform` (`SceneComponent.GetRelativeTransform` (`self.Floor`))))
  (bind _returnvalue_location_2 (`KismetMathLibrary.BreakTransform` (`SceneComponent.GetRelativeTransform` _floor)))
  (bind _returnvalue_location_3 (`KismetMathLibrary.BreakTransform` (`SceneComponent.GetRelativeTransform` _floor_2)))
  (bind _returnvalue_location_4 (`KismetMathLibrary.BreakTransform` (`SceneComponent.GetRelativeTransform` (`self.Floor`))))
  (bind _returnvalue_location_5 (`KismetMathLibrary.BreakTransform` (`SceneComponent.GetRelativeTransform` _floor_3)))
  (bind _returnvalue_location_6 (`KismetMathLibrary.BreakTransform` (`SceneComponent.GetRelativeTransform` (`self.Floor`))))
  (bind (_relativescale3d_x _relativescale3d_y) (`KismetMathLibrary.BreakVector` (`SceneComponent.RelativeScale3D` _floor)))
  (bind (_relativescale3d_x_2 _relativescale3d_y_2) (`KismetMathLibrary.BreakVector` (`SceneComponent.RelativeScale3D` _floor_2)))
  (bind (_relativescale3d_x_3 _relativescale3d_y_3) (`KismetMathLibrary.BreakVector` (`SceneComponent.RelativeScale3D` _floor_3)))
  (`|ExecutionSequence`
    (:`then_0`
      (set `local.WallLength` _gridsize)
      (set `local.WallThickness` (* _gridsize 0.1))
      (`SceneComponent.SetRelativeScale3D` (`self.Floor`) (`self.Size to Cube Scale` (`KismetMathLibrary.MakeVector` _walllength _walllength (`local.WallThickness`)))))
    (:`then_1`
      (`self.Walls` :!label _label))
    (:`then_2`
      (goto _label :!via `execute2`))
    (:`then_3`
      (goto _label :!via `execute3`))
    (:`then_4`
      (goto _label :!via `execute4`))
    (:`then_5`
      (`self.CeilingAndLight`))
    (:`then_6`
      (switch `/Game/_MyFiles/Blueprints/Enumeration/E_MazeType` (`self.MazeTypeEnum`)
        (:`NewEnumerator3`
          (if (not (>= (`KismetMathLibrary.RandomIntegerInRange` 0 10) 1))
            (`AddComponent|NODE_AddChildActorComponent-4` :`RelativeTransform` (`KismetMathLibrary.MakeTransform` (`KismetMathLibrary.MakeVector` (/ (* _relativescale3d_x_3 100.0) 2.0) (/ (* _relativescale3d_y_3 100.0) 2.0) (+ (.z _returnvalue_location_5) 180.0))))))
        (:`NewEnumerator4`
          (`AddComponent|NODE_AddChildActorComponent-6` :`RelativeTransform` (`KismetMathLibrary.MakeTransform` (`KismetMathLibrary.MakeVector` (/ (* _relativescale3d_x 100.0) 2.0) (/ (* _relativescale3d_y 100.0) 2.0) (+ (.z _returnvalue_location_2) 50.0)))))
        (:`NewEnumerator0`
          (`AddComponent|NODE_AddChildActorComponent-1` :`RelativeTransform` (`KismetMathLibrary.MakeTransform` (`KismetMathLibrary.MakeVector` (+ (.x _returnvalue_location) 75.0) (+ (.y _returnvalue_location) 75.0) (+ (.z _returnvalue_location) 50.0)))))
        (:`NewEnumerator1`
          (`AddComponent|NODE_AddChildActorComponent-2` :`RelativeTransform` (`KismetMathLibrary.MakeTransform` (`KismetMathLibrary.MakeVector` (+ (.x _returnvalue_location_6) 75.0) (+ (.y _returnvalue_location_6) 75.0) (+ (.z _returnvalue_location_6) 50.0)))))
        (:`NewEnumerator2`
          (`AddComponent|NODE_AddChildActorComponent-3` :`RelativeTransform` (`KismetMathLibrary.MakeTransform` (`KismetMathLibrary.MakeVector` (+ (.x _returnvalue_location_4) 50.0) (+ (.y _returnvalue_location_4) 50.0) (+ (.z _returnvalue_location_4) 50.0)))))
        (:`NewEnumerator6`
          (`AddComponent|NODE_AddChildActorComponent-7` :`RelativeTransform` (`KismetMathLibrary.MakeTransform` (`KismetMathLibrary.MakeVector` (+ (/ (* _relativescale3d_x_2 100.0) 2.0) (`KismetMathLibrary.RandomFloatInRange` -175.0 175.0)) (+ (/ (* _relativescale3d_y_2 100.0) 2.0) (`KismetMathLibrary.RandomFloatInRange` -175.0 175.0)) (+ (.z _returnvalue_location_3) 55.0)))))))
    (:`then_7`
      (`self.Pillars` :!label _label_2))
    (:`then_8`
      (goto _label_2 :!via `execute2`))
    (:`then_9`
      (goto _label_2 :!via `execute3`))
    (:`then_10`
      (goto _label_2 :!via `execute4`))))