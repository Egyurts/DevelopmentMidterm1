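; BP_EndPoint is the finish trigger that handles the win when the player reaches it.
; On BeginPlay it caches the player's BP_ThirdPersonCharacter, and its Box overlap reacts only to that actor.
; The overlap clears the timer held by StartPoint, calls Win on the player's UI and turns the lights of every BP_Labrent actor green.
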(event `self.Box.OnComponentBeginOverlap`
  (params (OverlappedComponent :type "PrimitiveComponent Object Reference") (OtherActor :type "Actor Object Reference") (OtherComp :type "PrimitiveComponent Object Reference") (OtherBodyIndex :type Integer) (bFromSweep :type Boolean) (SweepResult :type "HitResult Structure (by ref)"))
  (if (== OtherActor (`self.Player`))
    (`KismetSystemLibrary.K2_ClearAndInvalidateTimerHandle` (`/Game/_MyFiles/Blueprints/BP_StartPoint.Timer` (`self.StartPoint`)))
    (`/Game/_MyFiles/WBP/WBP_InGameUI.Win` (`/Game/ThirdPerson/Blueprints/BP_ThirdPersonCharacter.UI` (stale `self.ReceiveBeginPlay` _output_get)))
    (bind _outactors (`GameplayStatics.GetAllActorsOfClass` "/Game/_MyFiles/Blueprints/BP_Labrent.BP_Labrent_C"))
    (for _array_element _outactors
      (`/Game/_MyFiles/Blueprints/BP_Labrent.Change Light Color(Green)` _array_element))))

(event `self.ReceiveBeginPlay`
  (bind _asbp_third_person_character (cast `/Game/ThirdPerson/Blueprints/BP_ThirdPersonCharacter` (`GameplayStatics.GetPlayerCharacter` 0)))
  (bind _output_get (set `self.Player` _asbp_third_person_character)))

(fn `UserConstructionScript`)